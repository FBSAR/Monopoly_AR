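; BP_CardPath is a placeable actor that animates a Chance card flip in the AR Monopoly game.
; FlipCard plays a timeline whose alpha moves the card along the CardPath spline, then immediately overwrites that transform with a lerp between two stored card transforms.
; A separate Update function snaps the card to the spline's start at a small scale, using world-space location as relative location.
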(event Custom|FlipCard
  (bind _cardpath (Variables|Default|GetCardPath))
  (bind _flipanim (Timeline|Timeline_1 Play)
    (:Update
      (Transformation|SetRelativeTransform (Variables|Default|GetChanceCard) (Math|Transform|MakeTransform (Spline|GetLocationatDistanceAlongSpline _cardpath (Math|Float|Lerp 0.0 (Spline|GetSplineLength (Variables|Default|GetCardPath)) _flipanim) "Local") (Spline|GetRotationatDistanceAlongSpline _cardpath (Math|Float|Lerp 0.0 (Spline|GetSplineLength (Variables|Default|GetCardPath)) _flipanim) "Local") "1.063646,0.087409,0.778481") false false)
      (Transformation|SetRelativeTransform (Variables|Default|GetChanceCard) (Math|Transform|Lerp(Transform) (Variables|Default|GetCardTransform) (Variables|Default|GetCardTransform2) _flipanim) false false))))

(event EventBeginPlay
  (Utilities|FlowControl|Sequence
    (:then_0
      (Actor|GetActorOfClass "BP_CardPath_C"))))

(event EventTick
  (params (DeltaSeconds :type Float%20%28single-precision%29)))

(fn ConstructionScript)

(fn Update
  (bind _cardpath (Variables|Default|GetCardPath))
  (Transformation|SetRelativeTransform (Variables|Default|GetChanceCard) (Math|Transform|MakeTransform (Spline|GetLocationatDistanceAlongSpline _cardpath 0.0 "World") (Spline|GetRotationatDistanceAlongSpline _cardpath 0.0 "Local") "0.098301,0.087409,0.092960") false false)
  (return false))