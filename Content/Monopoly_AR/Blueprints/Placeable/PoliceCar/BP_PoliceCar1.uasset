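; BP_PoliceCar1 is a police car for the Monopoly AR game that starts hidden and drives along a BP_Track spline.
; MoveObject runs a timeline, scaled to a set duration, that moves the actor along the spline and reveals it, calling the siren sound every update.
; A second timeline animates red and blue light intensity together.
; The car mesh hides shortly after the run finishes; a FlipFlop light toggle is unconnected.
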(event Custom|Move%20Object
  (bind _spline_ref (Variables|Default|GetSpline%20Ref))
  (bind _spline (Variables|/Game/Monopoly_AR/Blueprints/Placeable/BP_Track.BP_Track_C|GetSpline _spline_ref))
  (Components|Timeline|SetPlayRate (Variables|Default|GetMove%20Object%20T) (/ 1.0 (Variables|Default|GetTime%20To%20Complete%20%28In%20Seconds%29)))
  (Utilities|FlowControl|Sequence
    (:then_0
      (bind _move_track (Timeline|Move%20Object%20T Play)
        (:Update
          (Transformation|SetActorTransform (Math|Transform|MakeTransform (Spline|GetLocationatDistanceAlongSpline _spline (Math|Float|Lerp 0.0 (Spline|GetSplineLength (Variables|/Game/Monopoly_AR/Blueprints/Placeable/BP_Track.BP_Track_C|GetSpline (Variables|Default|GetSpline%20Ref))) _move_track) "World") (Spline|GetRotationatDistanceAlongSpline _spline (Math|Float|Lerp 0.0 (Spline|GetSplineLength (Variables|/Game/Monopoly_AR/Blueprints/Placeable/BP_Track.BP_Track_C|GetSpline (Variables|Default|GetSpline%20Ref))) _move_track) "Local") "1.000000,1.000000,1.000000"))
          (Rendering|SetVisibility (Variables|Default|GetDefaultSceneRoot) true true)
          (Audio|PlaySound2D "/Game/Monopoly_AR/Blueprints/Placeable/PoliceCar/Siren_sounds.Siren_sounds" 0.1 1.0 0.0 0 0))
        (:Finished
          (Utilities|FlowControl|Delay 2.0)
          (Rendering|SetVisibility (Variables|Default|GetCar) false true))))
    (:then_1
      (bind _lightintensity (Timeline|PoliceLightAnimation Play)
        (:Update
          (Rendering|Components|Light|SetIntensity (Variables|Default|GetRedLight) _lightintensity)
          (Rendering|Components|Light|SetIntensity (Variables|Default|GetBlueLight) _lightintensity))))))

(event EventBeginPlay
  (bind _returnvalue (Actor|GetActorOfClass "/Game/Monopoly_AR/Blueprints/Placeable/BP_Track.BP_Track_C"))
  (Variables|Default|SetSpline%20Ref _returnvalue)
  (Rendering|SetVisibility (Variables|Default|GetDefaultSceneRoot) false true))

(event EventTick
  (params (DeltaSeconds :type Float%20%28single-precision%29)))

(fn ConstructionScript)